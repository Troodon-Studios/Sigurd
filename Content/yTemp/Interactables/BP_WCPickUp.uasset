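; BP_WCPickUp is a weapon pickup that gives its weapon to the player who picks it up.
; The construction script looks up the weapon item's data table row and sets the cube mesh to that row's display mesh.
; The PickUp event passes the weapon item to the player's CombatComponent to equip, then destroys the pickup actor.
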(event EventPickUp
  (params (Player :type BP%20Player%20Character%20Object%20Reference))
  (Class|CombatComponent|EquipWeapon (Variables|/Script/Sigurd.SigurdCharacter|GetCombatComponent Player) (Utilities|Struct|BreakSlots (Variables|Default|GetWeapon)))
  (Actor|DestroyActor))

(fn ConstructionScript
  (bind _weapon (Variables|Default|GetWeapon))
  (bind _item (Utilities|Struct|BreakSlots _weapon))
  (bind (_datatable _rowname) (Utilities|Struct|BreakDataTableRowHandle _item))
  (bind _returnvalue (Utilities|GetDataTableRow _datatable _rowname)
    (:then
      (Components|StaticMesh|SetStaticMesh (Variables|Default|GetCube) (.DisplayMesh (Utilities|Struct|BreakWeaponData _returnvalue))))))