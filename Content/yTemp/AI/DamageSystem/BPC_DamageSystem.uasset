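; BPC_DamageSystem is a component that resolves incoming hits on its owner as blocked, damaging or ignored.
; TakeDamage uses the CanBeDamaged macro to check death, invincibility and blocking against the DamageInfo flags.
; Damage goes through the owner's BP_ResourcesComponent, cached at BeginPlay, by amount and type.
; Event dispatchers report blocks with parry eligibility, death at zero health, and damage responses when interruptible or forced.
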(event EventBeginPlay
  (bind _returnvalue (Components|GetOwner))
  (bind _returnvalue_2 (Actor|GetComponentbyClass _returnvalue "/Game/Blueprints/PlayerCharacter/BP_ResourcesComponent.BP_ResourcesComponent_C"))
  (Utilities|IsValid _returnvalue_2
    (:Is%20Valid
      (Variables|Default|SetResourcesComponent _returnvalue_2))))

(fn TakeDamage
  (params (DamageInfo :type S%20Damage%20Info%20Structure))
  (bind (_amount _damagetype _damageresponse _shouddamageinvincible _canbeblocked _canbeparried _shouldforceinterrupt) (Utilities|Struct|BreakS_DamageInfo DamageInfo))
  (Utilities|CanbeDamaged _shouddamageinvincible _canbeblocked
    (:BlockDamage
      (Default|CallOnBlocked _canbeparried)
      (return false))
    (:DoDamage
      (Default|TakeDamagewithType (Variables|Default|GetResourcesComponent) _amount _damagetype)
      (if (<= (Variables|/Script/Sigurd.ResourcesComponent|GetcurrentHealth (Variables|Default|GetResourcesComponent)) 0.0)
        (Variables|Default|SetIsDead true)
        (Default|CallOnDeath)
        (return true)
        (elif (or (Variables|Default|GetIsInterruptuble) _shouldforceinterrupt)
          (Default|CallOnDamageResponse _damageresponse)
          (return true))))
    (:NoDamage
      (return false))))