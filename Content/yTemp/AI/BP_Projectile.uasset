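; Projectile actor that deals fire damage to whatever its capsule overlaps, other than its owner.
; Damage goes through a TakeDamageMessage call, and the projectile destroys itself whatever the result.
; A successful hit also spawns Niagara blood and a randomly sized spatter decal, placed by a visibility trace running upward from below the projectile.
; Overlapping the owner only prints a debug string.
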(event OnComponentBeginOverlap(Capsule)
  (params (OverlappedComponent :type Primitive%20Component%20Object%20Reference) (OtherActor :type Actor%20Object%20Reference) (OtherComp :type Primitive%20Component%20Object%20Reference) (OtherBodyIndex :type Integer) (bFromSweep :type Boolean) (SweepResult :type Hit%20Result%20Structure%20%28by%20ref%29))
  (bind _returnvalue (Transformation|GetActorLocation))
  (bind _returnvalue_2 (Transformation|GetActorLocation))
  (if (!= OtherActor (Components|GetOwner))
    (bind _wasdamaged (Class|BPIDamageable|TakeDamage(Message) OtherActor (Utilities|Struct|MakeS_DamageInfo (Variables|Default|GetDamageAmount) "/Game/Blueprints/DamageType/DT_FireDamage.DT_FireDamage" "NewEnumerator1")))
    (if _wasdamaged
      (Niagara|SpawnSystematLocation "/Game/VFX/NS_Blood.NS_Blood" _returnvalue)
      (bind _outhit (Collision|LineTraceByChannel (Math|Vector|MakeVector (.x _returnvalue_2) (.y _returnvalue_2) (- (.z _returnvalue_2) 1e+03)) _returnvalue "TraceTypeQuery1" false 0 "None"))
      (Rendering|Decal|SpawnDecalatLocation "/Game/Megascans/Decals/High_Velocity_Blood_Spatter_sfcsbflp/MI_High_Velocity_Blood_Spatter_sfcsbflp_2K.MI_High_Velocity_Blood_Spatter_sfcsbflp_2K" (Math|Conversions|ToVector(Float) (Math|Random|RandomFloatinRange 2e+01 7e+01)) (.ImpactPoint (Collision|BreakHitResult _outhit)) (Math|Conversions|RotationFromXVector (.Normal (Collision|BreakHitResult _outhit))) 0.0)
      (Actor|DestroyActor)
      (else
        (Actor|DestroyActor)))
    (else
      (Development|PrintString "AY"))))

(event EventBeginPlay)

(event Collision|EventActorBeginOverlap
  (params (OtherActor :type Actor%20Object%20Reference)))

(event EventTick
  (params (DeltaSeconds :type Float%20%28single-precision%29)))

(fn ConstructionScript)