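; BP_EnemyMele is a melee enemy character Blueprint that supplies melee-specific combat behavior for AI.
; Its Attack event reserves an attack token from the target, then triggers an attack through BPCombatComponent, printing a debug message if none is available.
; It also reports fixed attack and defend ranges and maps movement speed states to CharacterMovement walk speeds.
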(event EventBeginPlay
  (|CallParentFunction) ; This node is disabled and will not be called.\nDrag off pins to build functionality.
)

(event Collision|EventActorBeginOverlap
  (params (OtherActor :type Actor%20Object%20Reference)))

(event EventTick
  (params (DeltaSeconds :type Float%20%28single-precision%29)))

(event EventAttack
  (params (Target :type Actor%20Object%20Reference))
  (bind _success (Class|BPIDamageable|ReserveAttackToken(Message) Target 1))
  (if _success
    (Default|Attack (Variables|Default|GetBP_CombatComponent) "NewEnumerator0")
    (else
      (Development|PrintString "Not Enough Tokens"))))

(fn ConstructionScript
  (|CallParentFunction))

(fn GetIdealRange
  (return 1.5e+02 3.5e+02))

(fn SetMovementSpeed
  (params (Speed :type E_MovementSpeed%20Enum :default "NewEnumerator0"))
  (bind _output_get (Variables|/Script/Engine.CharacterMovementComponent|SetMaxWalkSpeed (Variables|Character|GetCharacterMovement) (Utilities|Select :Index Speed :NewEnumerator0 0.0 :NewEnumerator1 1e+02 :NewEnumerator3 2e+02 :NewEnumerator2 3.5e+02)))
  (return _output_get))