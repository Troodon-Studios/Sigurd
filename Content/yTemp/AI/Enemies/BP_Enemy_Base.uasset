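; BP_Enemy_Base is an enemy character base with combat, patrol and movement speed support.
; On BeginPlay it sets itself as owner of its BPCombatComponent and initializes that component with its start weapons.
; Its Attack event delegates to the combat component with a fixed attack enum value.
; It also exposes its patrol route and maps an idle-to-sprint speed enum onto the character's max walk speed.
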(event Custom|Attack
  (Default|Attack (Variables|Default|GetBP_CombatComponent) "NewEnumerator0"))

(event EventBeginPlay
  (bind _bp_combatcomponent (Variables|Default|GetBP_CombatComponent))
  (Variables|/Game/yTemp/AnimCombo/BP_CombatComponent.BP_CombatComponent_C|SetCharacterOwner _bp_combatcomponent self)
  (Default|InitializeWeapons _bp_combatcomponent (Variables|Default|GetStartWeapons)))

(fn ConstructionScript)

(fn GetPatrolRoute
  (return (Variables|AI|GetPatrolRoute)))

(fn SetMovementSpeed
  (params (Speed :type E_MovementSpeed%20Enum :default "NewEnumerator0"))
  (bind _output_get (Variables|/Script/Engine.CharacterMovementComponent|SetMaxWalkSpeed (Variables|Character|GetCharacterMovement) (Utilities|Select :Index Speed :NewEnumerator0 0.0 :NewEnumerator1 1e+02 :NewEnumerator3 3e+02 :NewEnumerator2 5e+02)))
  (return _output_get))