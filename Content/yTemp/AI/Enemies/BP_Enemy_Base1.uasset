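; Base AI enemy character that wires combat, resources and damage-system components to an AIC_Enemy_Base controller and health widget.
; Damageable hits route through the damage system, whose hit callback freezes the AI, spawns decals and plays a reaction before resuming combat.
; Death enables ragdoll physics and stops AI logic, while blocking uses montages and a state enum.
; Query functions expose health, patrol route, ranges, speed tiers and attack-token reservation.
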(event OnBlocked(BPC_DamageSystem)
  (params (CanBeParried :type Boolean))
  ;[1 1 1] Blocking Logic
  (Variables|Default|SetBlockingState "NewEnumerator2")
  (Animation|Montage|PlayMontage (Variables|Character|GetMesh) "/Game/Animation/Montages/AM_Parry_react.AM_Parry_react"))

(event Custom|StartBlock
  ;[1 1 1] Blocking Logic
  (Components|Movement|StopMovementImmediately (Variables|Character|GetCharacterMovement))
  (Variables|/Game/yTemp/AI/DamageSystem/BPC_DamageSystem.BPC_DamageSystem_C|SetIsBlocking (Variables|Default|GetBPC_DamageSystem) true)
  (Variables|Default|SetBlockingState "NewEnumerator1")
  (Animation|Montage|PlayMontage (Variables|Character|GetMesh) "/Game/Animation/Montages/AM_Parry_react.AM_Parry_react" 0.5
    (:OnCompleted
      (CallFunction|EndBlock :!label _label))
    (:OnInterrupted
      (if (Utilities|Enum|NotEqual(Enum) (Variables|Default|GetBlockingState) "NewEnumerator2")
        (goto _label)))))

(event Custom|EndBlock
  (bind _bp_combatcomponent (Variables|Default|GetBP_CombatComponent))
  ;[1 1 1] Blocking Logic
  (Variables|/Game/yTemp/AI/DamageSystem/BPC_DamageSystem.BPC_DamageSystem_C|SetIsBlocking (Variables|Default|GetBPC_DamageSystem) false)
  (Variables|Default|SetBlockingState "NewEnumerator0")
  (Default|CallOnBlockEnded)
  (Variables|/Game/yTemp/AnimCombo/BP_CombatComponent.BP_CombatComponent_C|SetcanStack _bp_combatcomponent true)
  (Variables|/Game/yTemp/AnimCombo/BP_CombatComponent.BP_CombatComponent_C|SetisAttacking _bp_combatcomponent false)
  (Variables|/Game/yTemp/AnimCombo/BP_CombatComponent.BP_CombatComponent_C|SetcanStack _bp_combatcomponent false))

(event Custom|Death
  (bind _mesh (Variables|Character|GetMesh))
  ;[1 1 1] DamageSystem Component
  (Physics|SetSimulatePhysics _mesh true)
  (Collision|SetCollisionEnabled _mesh "QueryAndPhysics")
  (AI|Logic|StopLogic (Variables|/Script/AIModule.AIController|GetBrainComponent (Variables|Default|GetAIController)) "Dead")
  (Development|SetHiddeninGame (Variables|Default|GetResources) true false)
  (Default|SetSateasDead (Variables|Default|GetAIController)))

(event Custom|Blocked
  (params (CanBeParried :type Boolean))
  ;[1 1 1] DamageSystem Component
  (Development|PrintString "Blocked"))

(event Custom|DamageResponse
  (params (DamageResponse :type E_DamageResponses%20Enum :default "NewEnumerator0") (DamageCauser :type Actor%20Object%20Reference))
  (bind _bp_combatcomponent (Variables|Default|GetBP_CombatComponent))
  ;[1 1 1] DamageSystem Component
  (Components|Movement|StopMovementImmediately (Variables|Character|GetCharacterMovement))
  (Default|SetStateasFrozen (Variables|Default|GetAIController))
  (bind (_impactpoint _normalrot) (CallFunction|GetDecalLocation self))
  (CallFunction|SpawnDecal "/Game/yTemp/VFX/Decals/DDT_Blood.DDT_Blood" _impactpoint _normalrot)
  (CallFunction|SpawnDecal (Variables|Default|GetDecalTable) _impactpoint _normalrot)
  (Variables|/Game/yTemp/AnimCombo/BP_CombatComponent.BP_CombatComponent_C|SetcanStack _bp_combatcomponent true)
  (Variables|/Game/yTemp/AnimCombo/BP_CombatComponent.BP_CombatComponent_C|SetisAttacking _bp_combatcomponent false)
  (Variables|/Game/yTemp/AnimCombo/BP_CombatComponent.BP_CombatComponent_C|SetcanStack _bp_combatcomponent false)
  (Animation|Montage|PlayMontage (Variables|Character|GetMesh) "/Game/Animation/Montages/AM_Damage.AM_Damage"
    (:OnCompleted
      _)
    (:OnInterrupted
      _))
  (Default|SetStateasCombat (Variables|Default|GetAIController) DamageCauser false))

(event Custom|Heal_1
  (params (Amount :type Float%20%28double-precision%29))
  (Class|ResourcesComponent|Heal (Variables|Default|GetBP_ResourcesComponent) Amount))

(event EventBeginPlay
  (bind _bp_combatcomponent (Variables|Default|GetBP_CombatComponent))
  (Variables|/Game/yTemp/AnimCombo/BP_CombatComponent.BP_CombatComponent_C|SetCharacterOwner _bp_combatcomponent self)
  (Default|InitializeWeapons _bp_combatcomponent (Variables|Default|GetStartWeapons))
  (bind _aswb_character_deb (Utilities|Casting|CastToWB_CharacterDeb (UserInterface|GetWidget (Variables|Default|GetResources))))
  (Variables|/Game/Widgets/Debug/WB_CharacterDeb.WB_CharacterDeb_C|SetResources%20Component _aswb_character_deb (Variables|Default|GetBP_ResourcesComponent))
  (bind _asaic_enemy_base (Utilities|Casting|CastToAIC_Enemy_Base (AI|GetAIController self)))
  (Variables|Default|SetAIController _asaic_enemy_base))

(event EventReturnAttackToken
  (params (Amount :type Integer))
  (Default|ReturnAttackToken (Variables|Default|GetBPC_DamageSystem) Amount))

(event Game|Damage|EventAnyDamage
  (params (Damage :type Float%20%28single-precision%29) (DamageType :type Damage%20Type%20Object%20Reference) (InstigatedBy :type Controller%20Object%20Reference) (DamageCauser :type Actor%20Object%20Reference))
  (Default|TakeDamagewithType (Variables|Default|GetBP_ResourcesComponent) DamageType Damage))

(fn ConstructionScript
  (bind _bpc_damagesystem (Variables|Default|GetBPC_DamageSystem))
  ;[1 1 1] Damage System Bindings
  (EventDispatchers|BindEventtoOnDeath _bpc_damagesystem (EventDispatchers|CreateEvent :!event Custom|Death))
  (EventDispatchers|BindEventtoOnBlocked _bpc_damagesystem (EventDispatchers|CreateEvent :!event Custom|Blocked))
  (EventDispatchers|BindEventtoOnDamageResponse _bpc_damagesystem (EventDispatchers|CreateEvent :!event Custom|DamageResponse)))

(fn GetCurrentHealth
  (return (Variables|/Script/Sigurd.ResourcesComponent|GetcurrentHealth (Variables|Default|GetBP_ResourcesComponent))))

(fn GetIdealRange
  (return 1.5e+02 3.5e+02))

(fn GetMaxHealth
  (return (Variables|/Script/Sigurd.ResourcesComponent|GetmaxHealth (Variables|Default|GetBP_ResourcesComponent))))

(fn GetPatrolRoute
  (return (Variables|AI|GetPatrolRoute)))

(fn Heal
  (params (Amount :type Float%20%28double-precision%29))
  (bind _bp_resourcescomponent (Variables|Default|GetBP_ResourcesComponent))
  (Class|ResourcesComponent|Heal _bp_resourcescomponent Amount)
  (return (Variables|/Script/Sigurd.ResourcesComponent|GetcurrentHealth _bp_resourcescomponent)))

(fn IsAttacking
  (return (Variables|/Game/yTemp/AnimCombo/BP_CombatComponent.BP_CombatComponent_C|GetisAttacking (Variables|Default|GetBP_CombatComponent))))

(fn ReserveAttackToken
  (params (Amount :type Integer))
  (bind _success (Default|ReserveAttackToken (Variables|Default|GetBPC_DamageSystem) Amount))
  (return _success))

(fn SetMovementSpeed
  (params (Speed :type E_MovementSpeed%20Enum :default "NewEnumerator0"))
  (bind _output_get (Variables|/Script/Engine.CharacterMovementComponent|SetMaxWalkSpeed (Variables|Character|GetCharacterMovement) (Utilities|Select :Index Speed :NewEnumerator0 0.0 :NewEnumerator1 1e+02 :NewEnumerator3 3e+02 :NewEnumerator2 5e+02)))
  (return _output_get))

(fn TakeDamageDamageable
  (params (DamageInfo :type S%20Damage%20Info%20Structure) (Damage%20Causer :type Actor%20Object%20Reference))
  (bind _wasdamaged (Default|TakeDamageSystem (Variables|Default|GetBPC_DamageSystem) DamageInfo Damage%20Causer))
  (return _wasdamaged))