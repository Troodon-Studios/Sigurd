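; Zombie enemy Blueprint that supplies the zombie's attack, combat ranges and movement speeds.
; The Attack event passes a single fixed attack type to the combat component.
; GetIdealRange returns constant attack and defend radii, while SetMovementSpeed maps a movement state to a slow max walk speed on CharacterMovement, always returning zero.
; BeginPlay, overlap and Tick are unused stubs.
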(event EventBeginPlay
  (|CallParentFunction) ; This node is disabled and will not be called.\nDrag off pins to build functionality.
)

(event Collision|EventActorBeginOverlap
  (params (OtherActor :type Actor%20Object%20Reference)))

(event EventTick
  (params (DeltaSeconds :type Float%20%28single-precision%29)))

(event EventAttack
  (Default|Attack (Variables|Default|GetBP_CombatComponent) "NewEnumerator0"))

(fn ConstructionScript
  (|CallParentFunction))

(fn GetIdealRange
  (return 1.5e+02 3.5e+02))

(fn SetMovementSpeed
  (params (Speed :type E_MovementSpeed%20Enum :default "NewEnumerator0"))
  (Variables|/Script/Engine.CharacterMovementComponent|SetMaxWalkSpeed (Variables|Character|GetCharacterMovement) (Utilities|Select :Index Speed :NewEnumerator0 0.0 :NewEnumerator1 5e+01 :NewEnumerator3 1e+02 :NewEnumerator2 1.5e+02))
  (return 0.0))