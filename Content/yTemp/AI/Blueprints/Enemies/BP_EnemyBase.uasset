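; Base enemy character that chases the player and performs an axe melee attack.
; On BeginPlay it uses AI MoveTo toward player character 0 within an acceptance radius.
; On reaching the player it plays the axe melee montage, waits briefly, and restarts the chase, forming a loop.
; Only a successful move continues the loop; a failed move has no handler.
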(event Custom|ChasePlayer
  (AI|AIMoveTo self "0, 0, 0" (Game|GetPlayerCharacter 0) (Variables|Default|GetAcceptanceRadius) false
    (:OnSuccess
      (CallFunction|Attack)
      (Utilities|FlowControl|Delay 0.2)
      (CallFunction|ChasePlayer))))

(event Custom|Attack
  (Animation|Montage|PlayMontage (Variables|Character|GetMesh) "/Game/Animation/Montages/Axe/AM_Axe-Mele.AM_Axe-Mele"))

(event EventBeginPlay
  (CallFunction|ChasePlayer))

(fn ConstructionScript)