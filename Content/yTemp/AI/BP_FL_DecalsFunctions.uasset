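; Decal function library that spawns randomized blood decals at a given location and rotation.
; SpawnDecal creates a dynamic instance of the blood decal material, has SetDecalParameters fill its textures from a random data table row with random texture rotation, then spawns it at random size.
; GetDecalLocation supplies an impact point and normal-based rotation by tracing on Visibility from below an actor up to its location.
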(fn SpawnDecal
  (params (Decaltable :type Data%20Table%20Object%20Reference) (Location :type Vector) (NormalRotation :type Rotator))
  (bind _returnvalue (Rendering|Material|CreateDynamicMaterialInstance 0 "/Game/Megascans/Decals/High_Velocity_Blood_Spatter_sfcsbflp/M_Decal_Blood_1.M_Decal_Blood_1" "None" :!class /Script/Engine.KismetMaterialLibrary))
  (bind _outputmaterial (CallFunction|SetDecalParameters 0 _returnvalue Decaltable))
  (Rendering|Decal|SpawnDecalatLocation 0 _outputmaterial (Math|Conversions|ToVector(Float) (Math|Random|RandomFloatinRange 4e+01 7e+01)) Location NormalRotation))

(fn SetDecalParameters
  (params (Material :type Material%20Instance%20Dynamic%20Object%20Reference) (Table :type Data%20Table%20Object%20Reference))
  (bind _outrownames (DataTable|GetDataTableRowNames Table))
  (bind _returnvalue (Utilities|GetDataTableRow Table (Utilities|Array|Get(acopy) _outrownames (Math|Random|RandomIntegerinRange 0 (Utilities|Array|Length _outrownames))))
    (:then
      (Rendering|Material|SetTextureParameterValue Material "Albedo" (.Albedo (Utilities|Struct|BreakS_DecalText _returnvalue)))
      (Rendering|Material|SetTextureParameterValue Material "Normal" (.Normal (Utilities|Struct|BreakS_DecalText _returnvalue)))
      (Rendering|Material|SetTextureParameterValue Material "DRO" (.DRO (Utilities|Struct|BreakS_DecalText _returnvalue)))
      (Rendering|Material|SetScalarParameterValue Material "TextRot" (Math|Random|RandomFloatinRange 0.0 1.0) :!class /Script/Engine.MaterialInstanceDynamic)
      (return Material))))

(fn GetDecalLocation
  (params (Actor :type Actor%20Object%20Reference))
  (bind _returnvalue (Transformation|GetActorLocation Actor))
  (bind _outhit (Collision|LineTraceByChannel 0 (Math|Vector|MakeVector (.x _returnvalue) (.y _returnvalue) (- (.z _returnvalue) 1e+03)) (Transformation|GetActorLocation Actor) "TraceTypeQuery1" false 0 "None"))
  (return (.ImpactPoint (Collision|BreakHitResult _outhit)) (Math|Conversions|RotationFromXVector (.Normal (Collision|BreakHitResult _outhit)))))