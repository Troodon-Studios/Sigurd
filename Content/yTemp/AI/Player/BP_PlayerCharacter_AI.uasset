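; Player character for mouse-aimed melee combat with weapon switching, dodge, parry, interaction and pickups.
; Each tick projects the cursor onto the ground plane for aiming; timelines turn attacks toward it and dash quick attacks at nearby targets.
; Combat, resources and damage-system components handle weapons, health and attack tokens, with hit gore and slow-motion ragdoll death.
; Debug keys switch elements and test enemy AI, noise and damage.
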(event OnComponentBeginOverlap(InteractableRadius)
  (params (OverlappedComponent :type Primitive%20Component%20Object%20Reference) (OtherActor :type Actor%20Object%20Reference) (OtherComp :type Primitive%20Component%20Object%20Reference) (OtherBodyIndex :type Integer) (bFromSweep :type Boolean) (SweepResult :type Hit%20Result%20Structure%20%28by%20ref%29))
  (Class|BPIInteract|ShowInterface(Message) OtherActor))

(event OnComponentEndOverlap(InteractableRadius)
  (params (OverlappedComponent :type Primitive%20Component%20Object%20Reference) (OtherActor :type Actor%20Object%20Reference) (OtherComp :type Primitive%20Component%20Object%20Reference) (OtherBodyIndex :type Integer))
  (Class|BPIInteract|HideInterface(Message) OtherActor))

(event OnComponentBeginOverlap(CapsuleComponent)
  (params (OverlappedComponent :type Primitive%20Component%20Object%20Reference) (OtherActor :type Actor%20Object%20Reference) (OtherComp :type Primitive%20Component%20Object%20Reference) (OtherBodyIndex :type Integer) (bFromSweep :type Boolean) (SweepResult :type Hit%20Result%20Structure%20%28by%20ref%29))
  (Class|BPIInteract|PickUp(Message) OtherActor (Variables|Default|GetBP_CombatComponent)))

(event Custom|DashToTarget
  ;[1 1 1] Dash To Target
  (if (and (Utilities|IsValid (Variables|Default|GetTarget)) (<= (Transformation|GetDistanceTo (Variables|Default|GetTarget)) 5e+02))
    (Variables|Default|SetCanAttack false)
    (Variables|Default|SetCanMove false)
    (Variables|Default|SetPrevLoc (Transformation|GetActorLocation))
    (Variables|Default|SetPrevRot (Transformation|GetActorRotation))
    (bind _blend (Timeline|Dash PlayFromStart)
      (:Update
        (Transformation|SetActorLocation (Math|Vector|MakeVector (.x (Math|Vector|Lerp(Vector) (Variables|Default|GetPrevLoc) (+ (* (Math|Vector|Normalize (- (Variables|Default|GetPrevLoc) (Transformation|GetActorLocation (Variables|Default|GetTarget)))) 175.0) (Transformation|GetActorLocation (Variables|Default|GetTarget))) _blend)) (.y (Math|Vector|Lerp(Vector) (Variables|Default|GetPrevLoc) (+ (* (Math|Vector|Normalize (- (Variables|Default|GetPrevLoc) (Transformation|GetActorLocation (Variables|Default|GetTarget)))) 175.0) (Transformation|GetActorLocation (Variables|Default|GetTarget))) _blend)) (.z (Variables|Default|GetPrevLoc))) true false)
        (Transformation|SetActorRotation (Math|Rotator|Lerp(Rotator) (Variables|Default|GetPrevRot) (Math|Interpolation|RInterpTo (Variables|Default|GetPrevRot) (Math|Rotator|FindLookatRotation (Variables|Default|GetPrevLoc) (Transformation|GetActorLocation (Variables|Default|GetTarget))) (Utilities|Time|GetWorldDeltaSeconds) 0.0) _blend))))))

(event Custom|RotateToCursor
  (bind _capsulecomponent (Variables|Default|GetCapsuleComponent))
  ;[1 1 1] Rotate To Mouse
  (Variables|Default|SetPrevRot (Transformation|GetActorRotation))
  (bind _blend (Timeline|Timeline PlayFromStart)
    (:Update
      (Transformation|SetWorldRotation _capsulecomponent (Math|Rotator|MakeRotator (.roll (Variables|Default|GetPrevRot)) (.pitch (Variables|Default|GetPrevRot)) (.yaw (Math|Rotator|Lerp(Rotator) (Variables|Default|GetPrevRot) (Math|Rotator|FindLookatRotation (Transformation|GetWorldLocation _capsulecomponent) (Variables|Default|GetMousePos)) _blend))) false false))))

(event Custom|Death
  (bind _mesh (Variables|Character|GetMesh))
  ;[1 1 1] DamageSystem Component
  (Development|PrintString "Dead")
  (Physics|SetSimulatePhysics _mesh true)
  (Collision|SetCollisionEnabled _mesh "QueryAndPhysics")
  (Input|DisableInput (Game|GetPlayerController 0))
  (Development|SetHiddeninGame (Variables|Default|GetResources) true false)
  (Camera|PlayWorldCameraShake "/Game/Blueprints/Other/BC_BigCameraShake.BC_BigCameraShake_C" (Transformation|GetActorLocation) 0.0 5e+03)
  (bind _time (Timeline|Slowmo Play)
    (:Update
      (Utilities|Time|SetGlobalTimeDilation _time))))

(event Custom|Blocked
  (params (CanBeParried :type Boolean))
  ;[1 1 1] DamageSystem Component
  (Development|PrintString "Blocked"))

(event Custom|DamageResponse
  (params (DamageResponse :type E_DamageResponses%20Enum :default "NewEnumerator0") (DamageCauser :type Actor%20Object%20Reference))
  ;[1 1 1] DamageSystem Component
  (Development|PrintString (Utilities|String|EnumtoString DamageResponse))
  (bind (_impactpoint _normalrot) (CallFunction|GetDecalLocation self))
  (CallFunction|SpawnDecal "/Game/yTemp/VFX/Decals/DDT_Blood.DDT_Blood" _impactpoint _normalrot)
  (CallFunction|SpawnDecal "/Game/yTemp/VFX/Decals/DDT_Bones.DDT_Bones" _impactpoint _normalrot)
  (Niagara|SpawnSystematLocation "/Game/VFX/NS_Blood.NS_Blood" (Transformation|GetActorLocation)))

(event Input|EnhancedActionEvents|EnhancedInputActionIA_Interact
  (params (ActionValue :type Boolean) (ElapsedSeconds :type Float%20%28double-precision%29) (TriggeredSeconds :type Float%20%28double-precision%29) (InputAction :type Input%20Action%20Object%20Reference :default "/Game/Input/Actions/IA_Interact.IA_Interact"))
  (:Started
    (bind _array_element (Utilities|Array|ForEachLoopwithBreak (Collision|GetOverlappingActors (Variables|Default|GetInteractableRadius) 0 :!class /Script/Engine.PrimitiveComponent) :!label _label)
      (:LoopBody
        (if (Utilities|DoesObjectImplementInterface _array_element "/Game/yTemp/Interactables/BPI_Interact.BPI_Interact_C")
          (Class|BPIInteract|Interact(Message) _array_element)
          (goto _label Break))))))

(event EventBeginPlay
  (Variables|/Script/Engine.PlayerController|SetbShowMouseCursor (Game|GetPlayerController 0) true)
  (bind _returnvalue (UserInterface|CreateWidget "/Game/yTemp/WFC_Maps/MiniMap/WB_MiniMap.WB_MiniMap_C"))
  (UserInterface|Viewport|AddtoViewport _returnvalue 0)
  (Variables|/Game/yTemp/AnimCombo/BP_CombatComponent.BP_CombatComponent_C|SetCharacterOwner (Variables|Default|GetBP_CombatComponent) self)
  (Default|InitializeWeapons (Variables|Default|GetBP_CombatComponent) (Variables|Default|GetStartWeapons))
  (bind _aswb_character_deb (Utilities|Casting|CastToWB_CharacterDeb (UserInterface|GetWidget (Variables|Default|GetResources))))
  (Variables|/Game/Widgets/Debug/WB_CharacterDeb.WB_CharacterDeb_C|SetResources%20Component _aswb_character_deb (Variables|Default|GetBP_ResourcesComponent)))

(event EventRun)

(event EventTick
  (params (DeltaSeconds :type Float%20%28single-precision%29))
  (CallFunction|RotateMousePointer)
  (CallFunction|UpdateBreath))

(event Game|Damage|EventAnyDamage
  (params (Damage :type Float%20%28single-precision%29) (DamageType :type Damage%20Type%20Object%20Reference) (InstigatedBy :type Controller%20Object%20Reference) (DamageCauser :type Actor%20Object%20Reference))
  (Default|TakeDamagewithType (Variables|Default|GetBP_ResourcesComponent) DamageType Damage))

(event EventReturnAttackToken
  (params (Amount :type Integer))
  (Default|ReturnAttackToken (Variables|Default|GetBPC_DamageSystem) Amount))

(event Input|KeyboardEvents|5
  (params (Key :type Key%20Structure :default "None"))
  ;[1 1 1] DEBUG
  (:Pressed
    (Default|ChangeElement (Variables|/Game/yTemp/AnimCombo/BP_CombatComponent.BP_CombatComponent_C|GetWeapon (Variables|Default|GetBP_CombatComponent)) "/Game/yTemp/Elements/ET_Water.ET_Water")))

(event Input|KeyboardEvents|X
  (params (Key :type Key%20Structure :default "None"))
  ;[1 1 1] DEBUG
  (:Pressed
    (bind _returnvalue (Actor|GetActorOfClass "/Game/yTemp/AI/Enemies/BP_Enemy.BP_Enemy_C"))
    (Class|AISenseDamage|ReportDamageEvent _returnvalue self 1.0 (Transformation|GetActorLocation) "0, 0, 0" "None")
    (Development|PrintString "Sending damage")))

(event Input|KeyboardEvents|1
  (params (Key :type Key%20Structure :default "None"))
  ;[1 1 1] DEBUG
  (:Pressed
    (bind _returnvalue (Actor|GetActorOfClass "/Game/yTemp/AI/Enemies/BP_Enemy.BP_Enemy_C"))
    (bind _asaic_enemy_base (Utilities|Casting|CastToAIC_Enemy_Base (AI|GetAIController _returnvalue)))
    (Utilities|FlowControl|FlipFlop
      (:A
        (Default|SetStateasCombat _asaic_enemy_base self false))
      (:B
        (Default|SetSateasPassive _asaic_enemy_base)))))

(event Input|KeyboardEvents|F
  (params (Key :type Key%20Structure :default "None"))
  (bind _returnvalue (Transformation|GetActorLocation))
  ;[1 1 1] DEBUG
  (:Pressed
    (Class|Actor|MakeNoise 1.0 0 _returnvalue 0.0 "None")
    (Effects|SpawnEmitteratLocation "/Game/zDeprecated/StarterContent/Particles/P_Explosion.P_Explosion" _returnvalue)
    (Audio|PlaySoundatLocation "/Game/zDeprecated/StarterContent/Audio/Explosion_Cue.Explosion_Cue" _returnvalue "0, 0, 0" 1.0 1.0 0.0 0 0 0 0)
    (Development|PrintString "Doing Noise")))

(event Input|KeyboardEvents|9
  (params (Key :type Key%20Structure :default "None"))
  ;[1 1 1] DEBUG
  (:Pressed
    (Variables|Default|SetMoveByClick (not (Variables|Default|GetMoveByClick)))
    (Variables|Default|SetCanMove true)))

(event Input|KeyboardEvents|8
  (params (Key :type Key%20Structure :default "None"))
  ;[1 1 1] DEBUG
  (:Pressed
    (Default|ChangeElement (Variables|/Game/yTemp/AnimCombo/BP_CombatComponent.BP_CombatComponent_C|GetWeapon (Variables|Default|GetBP_CombatComponent)) "/Game/yTemp/Elements/ET_Default.ET_Default")))

(event Input|KeyboardEvents|7
  (params (Key :type Key%20Structure :default "None"))
  ;[1 1 1] DEBUG
  (:Pressed
    (Default|ChangeElement (Variables|/Game/yTemp/AnimCombo/BP_CombatComponent.BP_CombatComponent_C|GetWeapon (Variables|Default|GetBP_CombatComponent)) "/Game/yTemp/Elements/ET_Fire.ET_Fire")))

(event Input|MouseEvents|MouseWheelDown
  (params (Key :type Key%20Structure :default "None"))
  ;[1 1 1] DEBUG
  (:Pressed
    (Default|Next/PrevWeapon (Variables|Default|GetBP_CombatComponent) true)))

(event Input|MouseEvents|MouseWheelUp
  (params (Key :type Key%20Structure :default "None"))
  ;[1 1 1] DEBUG
  (:Pressed
    (Default|Next/PrevWeapon (Variables|Default|GetBP_CombatComponent) false)))

(event Input|KeyboardEvents|6
  (params (Key :type Key%20Structure :default "None"))
  ;[1 1 1] DEBUG
  (:Pressed
    (Default|ChangeElement (Variables|/Game/yTemp/AnimCombo/BP_CombatComponent.BP_CombatComponent_C|GetWeapon (Variables|Default|GetBP_CombatComponent)) "/Game/yTemp/Elements/ET_Grass.ET_Grass")))

(event Input|KeyboardEvents|Q
  (params (Key :type Key%20Structure :default "None"))
  (bind _self self)
  (bind _capsulecomponent (Variables|Default|GetCapsuleComponent))
  (bind _returnvalue (Transformation|GetActorRotation _self))
  ;[1 1 1] DEBUG
  ;;[1 1 1] Dodge
  (:Pressed
    (Transformation|SetWorldRotation _capsulecomponent (Math|Rotator|MakeRotator (.roll _returnvalue) (.pitch _returnvalue) (.yaw (Math|Rotator|FindLookatRotation (Transformation|GetWorldLocation _capsulecomponent) (Variables|Default|GetMousePos)))) false false)
    (Default|Dodge (Variables|/Game/yTemp/AnimCombo/BP_CombatComponent.BP_CombatComponent_C|GetWeapon (Variables|Default|GetBP_CombatComponent)))))

(event Input|KeyboardEvents|E
  (params (Key :type Key%20Structure :default "None"))
  ;[1 1 1] DEBUG
  (:Pressed
    (Default|Parry (Variables|/Game/yTemp/AnimCombo/BP_CombatComponent.BP_CombatComponent_C|GetWeapon (Variables|Default|GetBP_CombatComponent)))))

(fn ConstructionScript
  (bind _bpc_damagesystem (Variables|Default|GetBPC_DamageSystem))
  ;[1 1 1] Damage System Bindings
  (EventDispatchers|BindEventtoOnDeath _bpc_damagesystem (EventDispatchers|CreateEvent :!event Custom|Death))
  (EventDispatchers|BindEventtoOnBlocked _bpc_damagesystem (EventDispatchers|CreateEvent :!event Custom|Blocked))
  (EventDispatchers|BindEventtoOnDamageResponse _bpc_damagesystem (EventDispatchers|CreateEvent :!event Custom|DamageResponse)))

(fn MeleAttack
  (Development|PrintString "Quick")
  (CallFunction|RotatetoCursor)
  (CallFunction|DashtoTarget)
  (Default|Attack (Variables|Default|GetBP_CombatComponent) "NewEnumerator0"))

(fn HeavyAttack
  (CallFunction|RotatetoCursor)
  (Default|Attack (Variables|Default|GetBP_CombatComponent) "NewEnumerator1"))

(fn RotateMousePointer
  (bind _returnvalue (Game|GetPlayerController 0))
  (bind _pointer (Variables|Default|GetPointer))
  (bind (_worldlocation _worlddirection) (Game|Player|ConvertMouseLocationToWorldSpace _returnvalue))
  (bind (_worldlocation_2 _worlddirection_2) (Game|Player|ConvertMouseLocationToWorldSpace _returnvalue))
  (bind _returnvalue_2 (/ (.z _worldlocation) (.z _worlddirection)))
  (bind _returnvalue_3 (* _worlddirection_2 _returnvalue_2))
  (bind _returnvalue_4 (* _returnvalue_3 -1))
  (bind _returnvalue_5 (+ _worldlocation_2 _returnvalue_4))
  (Transformation|SetWorldRotation _pointer (Math|Rotator|MakeRotator 0.0 0.0 (.yaw (Math|Rotator|FindLookatRotation (Transformation|GetWorldLocation _pointer) _returnvalue_5))) false false)
  (Variables|Default|SetMousePos _returnvalue_5))

(fn UpdateBreath
  (bind _returnvalue (Transformation|GetVelocity))
  (bind _returnvalue_2 (Math|Vector|VectorLength _returnvalue))
  (bind _returnvalue_3 (!= _returnvalue_2 0.0))
  (Effects|Components|ParticleSystem|SetEmitterEnable (Variables|Default|GetBreath) "Breath" _returnvalue_3)
  (if _returnvalue_3
    (Utilities|FlowControl|DoOnce false :!label _label
      (:Completed
        (Niagara|ResetSystem (Variables|Default|GetBreath))))
    (else
      (goto _label Reset))))

(fn GetCurrentHealth
  (return (Variables|/Script/Sigurd.ResourcesComponent|GetcurrentHealth (Variables|Default|GetBP_ResourcesComponent))))

(fn GetMaxHealth
  (return (Variables|/Script/Sigurd.ResourcesComponent|GetmaxHealth (Variables|Default|GetBP_ResourcesComponent))))

(fn Heal
  (params (Amount :type Float%20%28double-precision%29))
  (bind _bp_resourcescomponent (Variables|Default|GetBP_ResourcesComponent))
  (Class|ResourcesComponent|Heal _bp_resourcescomponent Amount)
  (return (Variables|/Script/Sigurd.ResourcesComponent|GetcurrentHealth _bp_resourcescomponent)))

(fn IsAttacking
  (return (Variables|/Game/yTemp/AnimCombo/BP_CombatComponent.BP_CombatComponent_C|GetisAttacking (Variables|Default|GetBP_CombatComponent))))

(fn ReserveAttackToken
  (params (Amount :type Integer))
  (bind _success (Default|ReserveAttackToken (Variables|Default|GetBPC_DamageSystem) Amount))
  (return _success))

(fn TakeDamageDamageable
  (params (DamageInfo :type S%20Damage%20Info%20Structure) (Damage%20Causer :type Actor%20Object%20Reference))
  (bind _wasdamaged (Default|TakeDamageSystem (Variables|Default|GetBPC_DamageSystem) DamageInfo Damage%20Causer))
  (return _wasdamaged))