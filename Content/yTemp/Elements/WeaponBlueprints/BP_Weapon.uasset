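; BP_Weapon is a weapon actor with an element type and quick and heavy attacks.
; ChangeElement, also run from the construction script, falls back to ET_Default when no valid element is given, then applies that element's overlay material to the mesh and its color to the trail effect.
; Quick plays the combo montage on the caster from a set section, while Heavy plays the heavy montage.
; BeginPlay and element changes print debug messages.
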(event EventBeginPlay
  (Development|PrintString "Im a weapon"))

(event Collision|EventActorBeginOverlap
  (params (OtherActor :type Actor%20Object%20Reference)))

(event EventTick
  (params (DeltaSeconds :type Float%20%28single-precision%29)))

(fn ConstructionScript
  (CallFunction|ChangeElement (Variables|Base|GetElementType)))

(fn ChangeElement
  (params (ElementType :type BPD%20Element%20Type%20Object%20Reference))
  (Utilities|FlowControl|Sequence
    (:then_0
      (if (Utilities|IsValid ElementType)
        (Variables|Base|SetElementType ElementType)
        (else
          (Variables|Base|SetElementType "/Game/yTemp/Elements/ET_Default.ET_Default"))))
    (:then_1
      (Rendering|Material|SetOverlayMaterial (Variables|Default|GetWeaponMesh) (Variables|/Game/yTemp/Elements/BPD_ElementType.BPD_ElementType_C|GetOverlayMaterial (Variables|Base|GetElementType)) :!class /Script/Engine.MeshComponent)
      (Niagara|SetNiagaraVariable(Vector3) (Variables|Default|GetTrailFX) "Element_Color" (Variables|/Game/yTemp/Elements/BPD_ElementType.BPD_ElementType_C|GetElementColor (Variables|Base|GetElementType)))
      (Development|PrintString "Element changed"))))

(fn Quick
  (params (Caster :type Character%20Object%20Reference))
  (Animation|PlayAnimMontage Caster (Variables|Montages|GetComboMontage) (Variables|Montages|GetPlayRate) (Variables|Montages|GetSection)))

(fn Heavy
  (params (Caster :type Character%20Object%20Reference))
  (Animation|PlayAnimMontage Caster (Variables|Montages|GetHeavyMontage) (Variables|Montages|GetPlayRate) "None"))