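; Breakable prop that shatters on overlap to reveal a floating reward mesh, with all three meshes set in the construction script.
; Overlap swaps the intact static mesh for a physics-simulated skeletal mesh and triggers Niagara sparkles.
; A fade timeline crossfades material opacity from debris to reward, then disables debris physics and collision.
; A looping timeline offsets and spins the reward, which starts invisible and has no pickup logic here.
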(event OnComponentBeginOverlap(StaticMesh)
  (params (OverlappedComponent :type Primitive%20Component%20Object%20Reference) (OtherActor :type Actor%20Object%20Reference) (OtherComp :type Primitive%20Component%20Object%20Reference) (OtherBodyIndex :type Integer) (bFromSweep :type Boolean) (SweepResult :type Hit%20Result%20Structure%20%28by%20ref%29))
  (bind _skeletalmesh (Variables|Default|GetSkeletalMesh))
  (bind _skeletalmesh_2 (Variables|Default|GetSkeletalMesh))
  (if (!= OtherActor self)
    (Collision|SetCollisionEnabled (Variables|Default|GetStaticMesh) "NoCollision")
    (Physics|SetSimulatePhysics (Variables|Default|GetSkeletalMesh) true)
    (Development|SetHiddeninGame (Variables|Default|GetStaticMesh) true true)
    (Development|SetHiddeninGame _skeletalmesh false true)
    (Collision|SetCollisionEnabled _skeletalmesh "QueryAndPhysics")
    (Components|Activation|Activate (Variables|Default|GetNS_Sparkles) false)
    (bind _outopacity (Timeline|FadeOpacity Play)
      (:Update
        (Rendering|Material|SetScalarParameterValueonMaterials (Variables|Default|GetSkeletalMesh) "Opacity" _outopacity)
        (Rendering|Material|SetScalarParameterValueonMaterials (Variables|Default|GetReward) "Opacity" (- 1.0 _outopacity)))
      (:Finished
        (Physics|SetSimulatePhysics _skeletalmesh_2 false)
        (Collision|SetCollisionEnabled _skeletalmesh_2 "NoCollision")))))

(event EventBeginPlay
  (bind _reward (Variables|Default|GetReward))
  (Development|SetHiddeninGame (Variables|Default|GetStaticMesh) false true)
  (Development|SetHiddeninGame (Variables|Default|GetSkeletalMesh) true true)
  (Collision|SetCollisionEnabled (Variables|Default|GetSkeletalMesh) "NoCollision")
  (Rendering|Material|SetScalarParameterValueonMaterials (Variables|Default|GetReward) "Opacity" 0.0)
  (bind _z_pos (Timeline|Timeline Play)
    (:Update
      (Transformation|AddLocalOffset _reward (Math|Vector|MakeVector 0.0 0.0 _z_pos) false false)
      (Transformation|AddRelativeRotation _reward (Math|Rotator|MakeRotator 0.0 0.0 1.0) false false))
    (:Finished
      (Utilities|FlowControl|DelayUntilNextTick)
      (Timeline|Timeline PlayFromStart))))

(fn ConstructionScript
  (Components|StaticMesh|SetStaticMesh (Variables|Default|GetStaticMesh) (Variables|Default|GetST_Mesh))
  (Components|SkeletalMesh|SetSkeletalMeshAsset (Variables|Default|GetSkeletalMesh) (Variables|Default|GetSK_Mesh))
  (Components|StaticMesh|SetStaticMesh (Variables|Default|GetReward) (Variables|Default|GetRewardMesh)))