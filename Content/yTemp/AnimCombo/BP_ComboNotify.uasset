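; BP_ComboNotify is an animation notify state that opens a combo input window during attack animations.
; On begin it sets CanStack on the owner's BP_CombatComponent.
; On end it clears CanStack and IsAttacking, then checks the Stacked attack value.
; Depending on that value, it either sets the weapon's Section from the notify and calls Attack with the stacked input, or sets Section to ResetAttack.
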(fn ReceivedNotifyBegin
  (params (MeshComp :type Skeletal%20Mesh%20Component%20Object%20Reference) (Animation :type Anim%20Sequence%20Base%20Object%20Reference) (TotalDuration :type Float%20%28single-precision%29) (EventReference :type Anim%20Notify%20Event%20Reference%20Structure%20%28by%20ref%29))
  (Variables|/Game/yTemp/AnimCombo/BP_CombatComponent.BP_CombatComponent_C|SetcanStack (Actor|GetComponentbyClass (Components|GetOwner MeshComp) "/Game/yTemp/AnimCombo/BP_CombatComponent.BP_CombatComponent_C") true)
  (return false))

(fn ReceivedNotifyEnd
  (params (MeshComp :type Skeletal%20Mesh%20Component%20Object%20Reference) (Animation :type Anim%20Sequence%20Base%20Object%20Reference) (EventReference :type Anim%20Notify%20Event%20Reference%20Structure%20%28by%20ref%29))
  (bind _returnvalue (Components|GetOwner MeshComp))
  (bind _returnvalue_2 (Actor|GetComponentbyClass _returnvalue "/Game/yTemp/AnimCombo/BP_CombatComponent.BP_CombatComponent_C"))
  (bind _stacked (Variables|/Game/yTemp/AnimCombo/BP_CombatComponent.BP_CombatComponent_C|Getstacked _returnvalue_2))
  (bind _weapon (Variables|/Game/yTemp/AnimCombo/BP_CombatComponent.BP_CombatComponent_C|GetWeapon _returnvalue_2))
  (bind _output_get (Variables|/Game/yTemp/AnimCombo/BP_CombatComponent.BP_CombatComponent_C|SetisAttacking _returnvalue_2 false))
  (Variables|/Game/yTemp/AnimCombo/BP_CombatComponent.BP_CombatComponent_C|SetcanStack _returnvalue_2 _output_get)
  (if (Utilities|Enum|NotEqual(Enum) _stacked "NewEnumerator2")
    (Variables|/Game/yTemp/Elements/WeaponBlueprints/BP_Weapon.BP_Weapon_C|SetSection _weapon (Variables|Default|GetSection))
    (Default|Attack _returnvalue_2 _stacked)
    (return true)
    (else
      (Variables|/Game/yTemp/Elements/WeaponBlueprints/BP_Weapon.BP_Weapon_C|SetSection _weapon (LocalVariables|GetResetAttack))
      (return false))))