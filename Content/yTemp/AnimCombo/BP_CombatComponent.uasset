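; Combat component that gives its owning character a switchable axe, hammer and spear with quick and heavy attacks.
; InitializeWeapons spawns all three, attaches them to mesh sockets and shows only the first.
; Attack calls the active weapon's attack unless one is running, or buffers the input while stacking is allowed.
; ChangeWeapon works in two passes: storing the pending weapon and playing a montage, then swapping visibility when TmpSet is true.
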(event EventBeginPlay)

(event EventTick
  (params (DeltaSeconds :type Float%20%28single-precision%29)))

(fn Attack
  (params (Selection :type E_AttackType%20Enum :default "NewEnumerator0"))
  (bind _weapon (Variables|Default|GetWeapon))
  (if (Variables|Default|GetcanStack)
    (Variables|Default|Setstacked Selection)
    (elif (not (Variables|Default|GetisAttacking))
      (switch Utilities|FlowControl|Switch|SwitchonE_AttackType Selection
        (:NewEnumerator0
          (Default|Quick _weapon (Variables|Default|GetCharacterOwner)))
        (:NewEnumerator1
          (Default|Heavy _weapon (Variables|Default|GetCharacterOwner))))
      (Variables|Default|Setstacked "NewEnumerator2")
      (Variables|Default|SetisAttacking true))))

(fn ChangeWeapon
  (params (Tmp/Set :type Boolean) (NewWeaponIndex :type Integer))
  (bind _aviableweapons (Variables|Default|GetAviableWeapons))
  (bind _output (Utilities|Array|Get(acopy) _aviableweapons NewWeaponIndex))
  (if (Utilities|IsValid _output)
    (if Tmp/Set
      (Rendering|SetActorHiddenInGame (Variables|Default|GetWeapon) true)
      (bind _output_get (Variables|Default|SetWeapon (Variables|Default|GettmpWeapon)))
      (Rendering|SetActorHiddenInGame _output_get false)
      (else
        (Variables|Default|SettmpWeapon _output)
        (Animation|PlayAnimMontage (Variables|Default|GetCharacterOwner) "/Game/Animation/Montages/AM_WeaponChange.AM_WeaponChange" 1.0 "None")
        (return)))
    (else
      ;[1 1 1] Error print
      (Development|PrintString (Utilities|String|Append "Weapon " (Utilities|String|ToString(Integer) NewWeaponIndex) " is out of bounds/not aviable") true true "(R=1.000000,G=0.000000,B=0.000000,A=1.000000)" 2.0 "Error"))))

(fn InitializeWeapons
  (bind _returnvalue (Game|SpawnActorfromClass "/Game/yTemp/Elements/WeaponBlueprints/BP_Axe.BP_Axe_C" (Math|Transform|MakeTransform "0, 0, 0" "0, 0, 0" "1.000000,1.000000,1.000000") "Undefined" "MultiplyWithRoot" 0 0))
  (bind _returnvalue_2 (Game|SpawnActorfromClass "/Game/yTemp/Elements/WeaponBlueprints/BP_Hammer.BP_Hammer_C" (Math|Transform|MakeTransform "0, 0, 0" "0, 0, 0" "1.000000,1.000000,1.000000") "Undefined" "MultiplyWithRoot" 0 0))
  (bind _returnvalue_3 (Game|SpawnActorfromClass "/Game/yTemp/Elements/WeaponBlueprints/BP_Spear.BP_Spear_C" (Math|Transform|MakeTransform "0, 0, 0" "0, 0, 0" "1.000000,1.000000,1.000000") "Undefined" "MultiplyWithRoot" 0 0))
  (bind _output_get (Variables|Default|SetAviableWeapons (Utilities|Array|MakeArray _returnvalue _returnvalue_2 _returnvalue_3)))
  (for (_array_element _array_index) _output_get
    (Transformation|AttachComponentToComponent (Variables|/Script/Engine.Actor|GetRootComponent _array_element) (Variables|/Script/Engine.Character|GetMesh (Variables|Default|GetCharacterOwner)) (Variables|Default|GetSocketName) "KeepRelative" "KeepRelative" "KeepRelative" true)
    (Rendering|SetActorHiddenInGame _array_element (!= _array_index 0)))
  (Variables|Default|SetWeapon (Utilities|Array|Get(acopy) (Variables|Default|GetAviableWeapons))))