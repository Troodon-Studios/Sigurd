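; BP_EnemyRanged is a ranged enemy that attacks by throwing a spear projectile.
; On BeginPlay it passes its enemy token component to the WB_TokenCount widget held by its TokenCounter component.
; EventAttack plays the spear-throw montage at increased speed, and a montage notify spawns BP_Projectile at the actor's location and rotation, with the enemy as owner and instigator.
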(event EventBeginPlay
  (bind _aswb_token_count (Utilities|Casting|CastToWB_TokenCount (UserInterface|GetWidget (Variables|Default|GetTokenCounter))))
  (Variables|/Game/yTemp/UI/WB_TokenCount.WB_TokenCount_C|SetTokenComponent _aswb_token_count (Variables|Default|GetTokenComponent_Enemy)))

(event Collision|EventActorBeginOverlap
  (params (OtherActor :type Actor%20Object%20Reference)))

(event EventTick
  (params (DeltaSeconds :type Float%20%28single-precision%29)))

(event EventEventAttack
  (params (AttackTarget :type Actor%20Object%20Reference))
  (bind _returnvalue (Transformation|GetActorTransform))
  (bind _self self)
  (bind _notifyname (Animation|Montage|PlayMontage (Variables|Character|GetMesh) "/Game/Animation/Montages/AM_SpearThrow.AM_SpearThrow" 3.0)
    (:OnNotifyBegin
      (switch name _notifyname
        (:Throw
          (Game|SpawnActorfromClass "/Game/AI/BP_Projectile.BP_Projectile_C" (Math|Transform|MakeTransform (.location _returnvalue) (.rotation _returnvalue) "1.000000,1.000000,1.000000") "AlwaysSpawn" "MultiplyWithRoot" _self _self))))))

(fn ConstructionScript)