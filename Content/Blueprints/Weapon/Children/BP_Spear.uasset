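; Spear weapon, a child weapon Blueprint whose Quick attack is overridden, without calling the parent, to throw a projectile.
; ThrowSpear plays a sped-up throw montage on the owning character and spawns BP_Projectile on notify begin.
; BP_PlayerCharacter_AI owners aim toward their raised mouse position; others use actor rotation.
; Each projectile receives the weapon's damage as blockable, unparryable fire damage that forces an interrupt.
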(event Custom|ThrowSpear
  (bind _characterowner (Variables|Default|GetCharacterOwner))
  (bind _characterowner_2 (Variables|Default|GetCharacterOwner))
  (bind _damage (Variables|Default|GetDamage))
  (bind _returnvalue (Transformation|GetActorTransform _characterowner_2))
  (bind _s_damageinfo (Utilities|Struct|MakeS_DamageInfo _damage "/Game/Blueprints/DamageType/DT_FireDamage.DT_FireDamage" "NewEnumerator1" false true false true))
  (bind _notifyname (Animation|Montage|PlayMontage (Variables|/Script/Engine.Character|GetMesh _characterowner_2) "/Game/Animation/Montages/AM_SpearThrow.AM_SpearThrow" 3.0)
    (:OnNotifyBegin
      (switch name _notifyname
        (:Throw
          (bind _asbp_player_character_ai (Utilities|Casting|CastToBP_PlayerCharacter_AI _characterowner_2)
            (:then
              (bind _returnvalue_2 (Game|SpawnActorfromClass "/Game/yTemp/AI/BP_Projectile.BP_Projectile_C" (Math|Transform|MakeTransform (.location _returnvalue) (Math|Rotator|FindLookatRotation (.location _returnvalue) (Math|Vector|MakeVector (.x (Variables|/Game/yTemp/AI/Player/BP_PlayerCharacter_AI.BP_PlayerCharacter_AI_C|GetMousePos _asbp_player_character_ai)) (.y (Variables|/Game/yTemp/AI/Player/BP_PlayerCharacter_AI.BP_PlayerCharacter_AI_C|GetMousePos _asbp_player_character_ai)) (+ (.z (Variables|/Game/yTemp/AI/Player/BP_PlayerCharacter_AI.BP_PlayerCharacter_AI_C|GetMousePos _asbp_player_character_ai)) 1.5e+02))) "1.000000,1.000000,1.000000") "AlwaysSpawn" "MultiplyWithRoot" _characterowner _characterowner))
              (Variables|/Game/yTemp/AI/BP_Projectile.BP_Projectile_C|SetDamage%20Info _returnvalue_2 _s_damageinfo))
            (:CastFailed
              (bind _returnvalue_3 (Game|SpawnActorfromClass "/Game/yTemp/AI/BP_Projectile.BP_Projectile_C" (Math|Transform|MakeTransform (.location _returnvalue) (.rotation _returnvalue) "1.000000,1.000000,1.000000") "AlwaysSpawn" "MultiplyWithRoot" _characterowner _characterowner))
              (Variables|/Game/yTemp/AI/BP_Projectile.BP_Projectile_C|SetDamage%20Info _returnvalue_3 _s_damageinfo))))))))

(event EventBeginPlay
  (|CallParentFunction))

(event Collision|EventActorBeginOverlap
  (params (OtherActor :type Actor%20Object%20Reference))
  (|CallParentFunction OtherActor) ; This node is disabled and will not be called.\nDrag off pins to build functionality.
)

(event EventTick
  (params (DeltaSeconds :type Float%20%28single-precision%29))
  (|CallParentFunction DeltaSeconds) ; This node is disabled and will not be called.\nDrag off pins to build functionality.
)

(fn ConstructionScript
  (|CallParentFunction))

(fn Quick
  (CallFunction|ThrowSpear))