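; BP_Weapon is a melee weapon that plays its owning character's combat montages and damages other actors overlapping its capsule.
; Quick, Heavy, Parry and Dodge play montages at WeaponSpeed, with Dodge also launching the character forward, scaled by that speed.
; ChangeElement, run from the construction script, applies the element's overlay material and trail color, falling back to ET_Default.
; Capsule overlaps deal fixed damage, with no attack-state check.
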(event OnComponentBeginOverlap(Capsule)
  (params (OverlappedComponent :type Primitive%20Component%20Object%20Reference) (OtherActor :type Actor%20Object%20Reference) (OtherComp :type Primitive%20Component%20Object%20Reference) (OtherBodyIndex :type Integer) (bFromSweep :type Boolean) (SweepResult :type Hit%20Result%20Structure%20%28by%20ref%29))
  (if (!= OtherActor (Variables|Default|GetCharacterOwner))
    (Game|Damage|ApplyDamage OtherActor 5.0 0 0)))

(event EventBeginPlay
  (Development|PrintString "Im a weapon"))

(event Collision|EventActorBeginOverlap
  (params (OtherActor :type Actor%20Object%20Reference)))

(event EventTick
  (params (DeltaSeconds :type Float%20%28single-precision%29)))

(fn ConstructionScript
  (CallFunction|ChangeElement (Variables|Base|GetElementType)))

(fn ChangeElement
  (params (ElementType :type BPD%20Element%20Type%20Object%20Reference))
  (Utilities|FlowControl|Sequence
    (:then_0
      (if (Utilities|IsValid ElementType)
        (Variables|Base|SetElementType ElementType)
        (else
          (Variables|Base|SetElementType "/Game/yTemp/Elements/ET_Default.ET_Default"))))
    (:then_1
      (Rendering|Material|SetOverlayMaterial (Variables|Default|GetWeaponMesh) (Variables|/Game/yTemp/Elements/BPD_ElementType.BPD_ElementType_C|GetOverlayMaterial (Variables|Base|GetElementType)) :!class /Script/Engine.MeshComponent)
      (Niagara|SetNiagaraVariable(Vector3) (Variables|Default|GetTrailFX) "Element_Color" (Variables|/Game/yTemp/Elements/BPD_ElementType.BPD_ElementType_C|GetElementColor (Variables|Base|GetElementType)))
      (Development|PrintString "Element changed"))))

(fn Quick
  (Animation|PlayAnimMontage (Variables|Default|GetCharacterOwner) (Variables|Montages|GetComboMontage) (Variables|Montages|GetWeaponSpeed) (Variables|Montages|GetSection)))

(fn Heavy
  (Animation|PlayAnimMontage (Variables|Default|GetCharacterOwner) (Variables|Montages|GetHeavyMontage) (Variables|Montages|GetWeaponSpeed) "None"))

(fn Parry
  (Animation|PlayAnimMontage (Variables|Default|GetCharacterOwner) (Variables|Montages|GetParryMontage) (Variables|Montages|GetWeaponSpeed) "None"))

(fn Dodge
  (bind _characterowner (Variables|Default|GetCharacterOwner))
  (bind _returnvalue (Transformation|GetActorForwardVector _characterowner))
  (Animation|PlayAnimMontage _characterowner (Variables|Montages|GetDodgeMontage) (Variables|Montages|GetWeaponSpeed) "None")
  (Character|LaunchCharacter _characterowner (+ (* _returnvalue 8e+02) (* _returnvalue (* (Variables|Montages|GetWeaponSpeed) 2e+02))) false false))