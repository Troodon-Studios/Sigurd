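; Player character Blueprint for a mouse-aimed game, with world widgets for heavy melee and token count.
; Tick projects the cursor onto the Z=0 plane to aim a pointer and toggles breath particles with movement; the stored point drives instant (Q) or timeline-blended capsule turning.
; Overlaps and the Interact input send interface messages for prompts, pickups and interaction.
; F triggers a debug noise and explosion.
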(event OnComponentBeginOverlap(InteractableRadius)
  (params (OverlappedComponent :type Primitive%20Component%20Object%20Reference) (OtherActor :type Actor%20Object%20Reference) (OtherComp :type Primitive%20Component%20Object%20Reference) (OtherBodyIndex :type Integer) (bFromSweep :type Boolean) (SweepResult :type Hit%20Result%20Structure%20%28by%20ref%29))
  (Class|BPIInteract|ShowInterface(Message) OtherActor))

(event OnComponentEndOverlap(InteractableRadius)
  (params (OverlappedComponent :type Primitive%20Component%20Object%20Reference) (OtherActor :type Actor%20Object%20Reference) (OtherComp :type Primitive%20Component%20Object%20Reference) (OtherBodyIndex :type Integer))
  (Class|BPIInteract|HideInterface(Message) OtherActor))

(event OnComponentBeginOverlap(CapsuleComponent)
  (params (OverlappedComponent :type Primitive%20Component%20Object%20Reference) (OtherActor :type Actor%20Object%20Reference) (OtherComp :type Primitive%20Component%20Object%20Reference) (OtherBodyIndex :type Integer) (bFromSweep :type Boolean) (SweepResult :type Hit%20Result%20Structure%20%28by%20ref%29))
  (Class|BPIInteract|PickUp(Message) OtherActor (Variables|Default|GetCombatComponent))
  (Class|BPIInteract|PickWeapon(Message) OtherActor self))

(event Custom|RotateToCursor
  (bind _capsulecomponent (Variables|Default|GetCapsuleComponent))
  ;[1 1 1] Rotate To Mouse
  (Variables|Default|SetPrevRot (Transformation|GetActorRotation))
  (bind _blend (Timeline|Timeline PlayFromStart)
    (:Update
      (Transformation|SetWorldRotation _capsulecomponent (Math|Rotator|MakeRotator (.roll (Variables|Default|GetPrevRot)) (.pitch (Variables|Default|GetPrevRot)) (.yaw (Math|Rotator|Lerp(Rotator) (Variables|Default|GetPrevRot) (Math|Rotator|FindLookatRotation (Transformation|GetWorldLocation _capsulecomponent) (Variables|Default|GetMousePos)) _blend))) false false))))

(event Input|EnhancedActionEvents|EnhancedInputActionIA_Interact
  (params (ActionValue :type Boolean) (ElapsedSeconds :type Float%20%28double-precision%29) (TriggeredSeconds :type Float%20%28double-precision%29) (InputAction :type Input%20Action%20Object%20Reference :default "/Game/Input/Actions/IA_Interact.IA_Interact"))
  (:Started
    (bind _array_element (Utilities|Array|ForEachLoopwithBreak (Collision|GetOverlappingActors (Variables|Default|GetInteractableRadius) 0 :!class /Script/Engine.PrimitiveComponent) :!label _label)
      (:LoopBody
        (if (Utilities|DoesObjectImplementInterface _array_element "/Game/yTemp/Interactables/BPI_Interact.BPI_Interact_C")
          (Class|BPIInteract|Interact(Message) _array_element)
          (goto _label Break))))))

(event EventBeginPlay
  (bind _aswb_heavymele (Utilities|Casting|CastToWB_Heavymele (UserInterface|GetWidget (Variables|Default|GetHeavyMele))))
  (Variables|/Game/Widgets/Player/WB_Heavymele.WB_Heavymele_C|SetPlayer _aswb_heavymele self)
  (Variables|/Script/Engine.PlayerController|SetbShowMouseCursor (Game|GetPlayerController 0) true)
  (bind _returnvalue (Actor|GetActorOfClass "/Game/Blueprints/BP_HNS_Enemy.BP_HNS_Enemy_C"))
  (Variables|Default|SetTarget _returnvalue)
  (bind _aswb_token_count (Utilities|Casting|CastToWB_TokenCount (UserInterface|GetWidget (Variables|Default|GetTokenCounter))))
  (Variables|/Game/yTemp/UI/WB_TokenCount.WB_TokenCount_C|SetActor _aswb_token_count self))

(event EventTick
  (params (DeltaSeconds :type Float%20%28single-precision%29))
  (CallFunction|RotateMousePointer)
  (CallFunction|UpdateBreath))

(event Input|KeyboardEvents|F
  (params (Key :type Key%20Structure :default "None"))
  (bind _returnvalue (Transformation|GetActorLocation))
  ;[1 1 1] DEBUG
  (:Pressed
    (Class|Actor|MakeNoise 1.0 0 _returnvalue 0.0 "None")
    (Effects|SpawnEmitteratLocation "/Game/zDeprecated/StarterContent/Particles/P_Explosion.P_Explosion" _returnvalue)
    (Audio|PlaySoundatLocation "/Game/zDeprecated/StarterContent/Audio/Explosion_Cue.Explosion_Cue" _returnvalue "0, 0, 0" 1.0 1.0 0.0 0 0 0 0)))

(event Input|KeyboardEvents|E
  (params (Key :type Key%20Structure :default "None"))
  ;[1 1 1] DEBUG
)

(event Input|MouseEvents|MouseWheelDown
  (params (Key :type Key%20Structure :default "None"))
  ;[1 1 1] DEBUG
)

(event Input|MouseEvents|MouseWheelUp
  (params (Key :type Key%20Structure :default "None"))
  ;[1 1 1] DEBUG
)

(event Input|KeyboardEvents|Q
  (params (Key :type Key%20Structure :default "None"))
  (bind _self self)
  (bind _capsulecomponent (Variables|Default|GetCapsuleComponent))
  (bind _returnvalue (Transformation|GetActorRotation _self))
  ;[1 1 1] DEBUG
  ;;[1 1 1] Dodge
  (:Pressed
    (Transformation|SetWorldRotation _capsulecomponent (Math|Rotator|MakeRotator (.roll _returnvalue) (.pitch _returnvalue) (.yaw (Math|Rotator|FindLookatRotation (Transformation|GetWorldLocation _capsulecomponent) (Variables|Default|GetMousePos)))) false false)))

(fn ConstructionScript)

(fn RotateMousePointer
  (bind _returnvalue (Game|GetPlayerController 0))
  (bind _pointer (Variables|Default|GetPointer))
  (bind (_worldlocation _worlddirection) (Game|Player|ConvertMouseLocationToWorldSpace _returnvalue))
  (bind (_worldlocation_2 _worlddirection_2) (Game|Player|ConvertMouseLocationToWorldSpace _returnvalue))
  (bind _returnvalue_2 (/ (.z _worldlocation) (.z _worlddirection)))
  (bind _returnvalue_3 (* _worlddirection_2 _returnvalue_2))
  (bind _returnvalue_4 (* _returnvalue_3 -1))
  (bind _returnvalue_5 (+ _worldlocation_2 _returnvalue_4))
  (Transformation|SetWorldRotation _pointer (Math|Rotator|MakeRotator 0.0 0.0 (.yaw (Math|Rotator|FindLookatRotation (Transformation|GetWorldLocation _pointer) _returnvalue_5))) false false)
  (Variables|Default|SetMousePos _returnvalue_5))

(fn UpdateBreath
  (bind _returnvalue (Transformation|GetVelocity))
  (bind _returnvalue_2 (Math|Vector|VectorLength _returnvalue))
  (bind _returnvalue_3 (!= _returnvalue_2 0.0))
  (Effects|Components|ParticleSystem|SetEmitterEnable (Variables|Default|GetBreath) "Breath" _returnvalue_3)
  (if _returnvalue_3
    (Utilities|FlowControl|DoOnce false :!label _label
      (:Completed
        (Niagara|ResetSystem (Variables|Default|GetBreath))))
    (else
      (goto _label Reset))))