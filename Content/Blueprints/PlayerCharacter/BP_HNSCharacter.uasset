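; Top-down hack-and-slash player character that aims melee attacks at the mouse cursor and passes damage to a health component.
; Tick projects the cursor onto the ground to aim a pointer and toggles breath particles with movement.
; Weapon data assets supply the mesh, quick-combo montages and heavy montage, with timelines turning attacks toward the cursor or dashing to the enemy cached at BeginPlay.
; Debug keys swap axe and hammer data or toggle click-to-move.
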(event Custom|DashToTarget
  ;[1 1 1] Dash To Target
  (if (and (Utilities|IsValid (Variables|Default|GetTarget)) (<= (Transformation|GetDistanceTo (Variables|Default|GetTarget)) 5e+02))
    (Variables|Default|SetCanAttack false)
    (Variables|Default|SetCanMove false)
    (Variables|Default|SetPrevLoc (Transformation|GetActorLocation))
    (Variables|Default|SetPrevRot (Transformation|GetActorRotation))
    (bind _blend (Timeline|Dash PlayFromStart)
      (:Update
        (Transformation|SetActorLocation (Math|Vector|MakeVector (.x (Math|Vector|Lerp(Vector) (Variables|Default|GetPrevLoc) (+ (* (Math|Vector|Normalize (- (Variables|Default|GetPrevLoc) (Transformation|GetActorLocation (Variables|Default|GetTarget)))) 175.0) (Transformation|GetActorLocation (Variables|Default|GetTarget))) _blend)) (.y (Math|Vector|Lerp(Vector) (Variables|Default|GetPrevLoc) (+ (* (Math|Vector|Normalize (- (Variables|Default|GetPrevLoc) (Transformation|GetActorLocation (Variables|Default|GetTarget)))) 175.0) (Transformation|GetActorLocation (Variables|Default|GetTarget))) _blend)) (.z (Variables|Default|GetPrevLoc))) true false)
        (Transformation|SetActorRotation (Math|Rotator|Lerp(Rotator) (Variables|Default|GetPrevRot) (Math|Interpolation|RInterpTo (Variables|Default|GetPrevRot) (Math|Rotator|FindLookatRotation (Variables|Default|GetPrevLoc) (Transformation|GetActorLocation (Variables|Default|GetTarget))) (Utilities|Time|GetWorldDeltaSeconds) 0.0) _blend))))))

(event Custom|RotateToCursor
  (bind _capsulecomponent (Variables|Default|GetCapsuleComponent))
  ;[1 1 1] Rotate To Mouse
  (Variables|Default|SetPrevRot (Transformation|GetActorRotation))
  (bind _blend (Timeline|Timeline PlayFromStart)
    (:Update
      (Transformation|SetWorldRotation _capsulecomponent (Math|Rotator|MakeRotator (.roll (Variables|Default|GetPrevRot)) (.pitch (Variables|Default|GetPrevRot)) (.yaw (Math|Rotator|Lerp(Rotator) (Variables|Default|GetPrevRot) (Math|Rotator|FindLookatRotation (Transformation|GetWorldLocation _capsulecomponent) (Variables|Default|GetMousePos)) _blend))) false false))))

(event EventBeginPlay
  (bind _aswb_heavymele (Utilities|Casting|CastToWB_Heavymele (UserInterface|GetWidget (Variables|Default|GetHeavyMele))))
  (Variables|/Game/Widgets/HNS_Sigurd/WB_Heavymele.WB_Heavymele_C|SetPlayer _aswb_heavymele self)
  (Variables|/Script/Engine.PlayerController|SetbShowMouseCursor (Game|GetPlayerController 0) true)
  (bind _returnvalue (Actor|GetActorOfClass "/Game/Blueprints/BP_HNS_Enemy.BP_HNS_Enemy_C"))
  (Variables|Default|SetTarget _returnvalue)
  (bind _returnvalue_2 (UserInterface|CreateWidget "/Game/Widgets/Debug/WB_ScreenDeb.WB_ScreenDeb_C"))
  (UserInterface|Viewport|AddtoViewport _returnvalue_2 0)
  (Utilities|Casting|CastToWB_CharacterDeb (UserInterface|GetWidget (Variables|Default|GetDebug))))

(event Collision|EventActorBeginOverlap
  (params (OtherActor :type Actor%20Object%20Reference)))

(event EventTick
  (params (DeltaSeconds :type Float%20%28single-precision%29))
  (CallFunction|RotateMousePointer)
  (CallFunction|UpdateBreath))

(event Game|Damage|EventAnyDamage
  (params (Damage :type Float%20%28single-precision%29) (DamageType :type Damage%20Type%20Object%20Reference) (InstigatedBy :type Controller%20Object%20Reference) (DamageCauser :type Actor%20Object%20Reference))
  (Default|TakeDamagewithType (Variables|Default|GetBP_HealthComponent) DamageType Damage))

(event Input|KeyboardEvents|5
  (params (Key :type Key%20Structure))
  ;[1 1 1] DEBUG
)

(event Input|KeyboardEvents|6
  (params (Key :type Key%20Structure))
  ;[1 1 1] DEBUG
)

(event Input|KeyboardEvents|9
  (params (Key :type Key%20Structure))
  ;[1 1 1] DEBUG
  (:Pressed
    (Variables|Default|SetMoveByClick (not (Variables|Default|GetMoveByClick)))
    (Variables|Default|SetCanMove true)))

(event Input|KeyboardEvents|8
  (params (Key :type Key%20Structure))
  ;[1 1 1] DEBUG
  (:Pressed
    (bind _output_get (Variables|Default|SetWeaponData "/Game/Blueprints/Weapons/DA_Axe.DA_Axe"))
    (Variables|/Game/Blueprints/Weapons/BCD_Weapon.BCD_Weapon_C|SetActualAnim _output_get 0)
    (Animation|PlayAnimMontage "/Game/Animation/Montages/AM_WeaponChange.AM_WeaponChange" 2.0 "None")))

(event Input|KeyboardEvents|7
  (params (Key :type Key%20Structure))
  ;[1 1 1] DEBUG
  (:Pressed
    (bind _output_get (Variables|Default|SetWeaponData "/Game/Blueprints/Weapons/DA_Hammer.DA_Hammer"))
    (Variables|/Game/Blueprints/Weapons/BCD_Weapon.BCD_Weapon_C|SetActualAnim _output_get 0)
    (Animation|PlayAnimMontage "/Game/Animation/Montages/AM_WeaponChange.AM_WeaponChange" 2.0 "None")))

(fn ConstructionScript
  (CallFunction|ChangeWeapon))

(fn MeleAttack
  (bind _weapondata (Variables|Default|GetWeaponData))
  (bind _quickanim (Variables|/Game/Blueprints/Weapons/BCD_Weapon.BCD_Weapon_C|GetQuickAnim _weapondata))
  (CallFunction|RotatetoCursor)
  (CallFunction|DashtoTarget)
  (Animation|PlayAnimMontage (Utilities|Array|Get(acopy) _quickanim (Variables|/Game/Blueprints/Weapons/BCD_Weapon.BCD_Weapon_C|GetActualAnim _weapondata)) 1.0 "None")
  (Math|Integer|IncrementInt (Variables|/Game/Blueprints/Weapons/BCD_Weapon.BCD_Weapon_C|GetActualAnim (Variables|Default|GetWeaponData))
    (:%20%20
      (if (== (Variables|/Game/Blueprints/Weapons/BCD_Weapon.BCD_Weapon_C|GetActualAnim (Variables|Default|GetWeaponData)) (Utilities|Array|Length _quickanim))
        (Variables|/Game/Blueprints/Weapons/BCD_Weapon.BCD_Weapon_C|SetActualAnim (Variables|Default|GetWeaponData) 0)))))

(fn HeavyAttack
  (CallFunction|RotatetoCursor)
  (Animation|PlayAnimMontage (Variables|/Game/Blueprints/Weapons/BCD_Weapon.BCD_Weapon_C|GetHeavyAnim (Variables|Default|GetWeaponData)) 2.0 "None"))

(fn RotateMousePointer
  (bind _returnvalue (Game|GetPlayerController 0))
  (bind _pointer (Variables|Default|GetPointer))
  (bind (_worldlocation _worlddirection) (Game|Player|ConvertMouseLocationToWorldSpace _returnvalue))
  (bind (_worldlocation_2 _worlddirection_2) (Game|Player|ConvertMouseLocationToWorldSpace _returnvalue))
  (bind _returnvalue_2 (/ (.z _worldlocation) (.z _worlddirection)))
  (bind _returnvalue_3 (* _worlddirection_2 _returnvalue_2))
  (bind _returnvalue_4 (* _returnvalue_3 -1))
  (bind _returnvalue_5 (+ _worldlocation_2 _returnvalue_4))
  (Transformation|SetWorldRotation _pointer (Math|Rotator|MakeRotator 0.0 0.0 (.yaw (Math|Rotator|FindLookatRotation (Transformation|GetWorldLocation _pointer) _returnvalue_5))) false false)
  (Variables|Default|SetMousePos _returnvalue_5))

(fn ChangeWeapon
  (Components|SkeletalMesh|SetSkeletalMeshAsset (Variables|Default|GetWeaponMesh) (Variables|/Game/Blueprints/Weapons/BCD_Weapon.BCD_Weapon_C|GetMesh (Variables|Default|GetWeaponData))))

(fn UpdateBreath
  (bind _returnvalue (Transformation|GetVelocity))
  (bind _returnvalue_2 (Math|Vector|VectorLength _returnvalue))
  (bind _returnvalue_3 (!= _returnvalue_2 0.0))
  (Effects|Components|ParticleSystem|SetEmitterEnable (Variables|Default|GetBreath) "Breath" _returnvalue_3)
  (if _returnvalue_3
    (Utilities|FlowControl|DoOnce false :!label _label
      (:Completed
        (Niagara|ResetSystem (Variables|Default|GetBreath))))
    (else
      (goto _label Reset))))

(fn MeleAttack2
  (bind _weapondata (Variables|Default|GetWeaponData))
  (bind _quickanim (Variables|/Game/Blueprints/Weapons/BCD_Weapon.BCD_Weapon_C|GetQuickAnim _weapondata))
  (Animation|PlayAnimMontage (Utilities|Array|Get(acopy) _quickanim (Variables|/Game/Blueprints/Weapons/BCD_Weapon.BCD_Weapon_C|GetActualAnim _weapondata)) 2.0 "None")
  (Math|Integer|IncrementInt (Variables|/Game/Blueprints/Weapons/BCD_Weapon.BCD_Weapon_C|GetActualAnim (Variables|Default|GetWeaponData))
    (:%20%20
      (if (== (Variables|/Game/Blueprints/Weapons/BCD_Weapon.BCD_Weapon_C|GetActualAnim (Variables|Default|GetWeaponData)) (Utilities|Array|Length _quickanim))
        (Variables|/Game/Blueprints/Weapons/BCD_Weapon.BCD_Weapon_C|SetActualAnim (Variables|Default|GetWeaponData) 0)))))