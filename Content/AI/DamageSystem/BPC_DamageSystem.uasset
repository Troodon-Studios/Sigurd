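; BPC_DamageSystem is an actor component that resolves incoming hits and tracks attack tokens for its owner.
; CanBeDamaged routes each hit to block, damage or no damage using death, invincibility and blocking state plus DamageInfo overrides.
; Damage goes to the owner's HealthComponent, then fires death or, if interruptible or forced, damage response events; blocks report parryability.
; A simple token counter supports reserving and returning attack tokens.
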(event EventBeginPlay
  (bind _returnvalue (Components|GetOwner))
  (bind _returnvalue_2 (Actor|GetComponentbyClass _returnvalue "/Script/Sigurd.HealthComponent"))
  (Utilities|IsValid _returnvalue_2
    (:Is%20Valid
      (Variables|Default|SetHealthComponent _returnvalue_2))))

(fn TakeDamageSystem
  (params (DamageInfo :type S%20Damage%20Info%20Structure) (DamageCauser :type Actor%20Object%20Reference))
  (bind (_amount _damagetype _damageresponse _shouddamageinvincible _canbeblocked _canbeparried _shouldforceinterrupt) (Utilities|Struct|BreakS_DamageInfo DamageInfo))
  (Utilities|CanbeDamaged _shouddamageinvincible _canbeblocked
    (:BlockDamage
      (Default|CallOnBlocked _canbeparried)
      (return false))
    (:DoDamage
      (Class|HealthComponent|TakeDamagewithType (Variables|Default|GetHealthComponent) _damagetype _amount)
      (if (<= (Variables|/Script/Sigurd.HealthComponent|GetCurrentHealth (Variables|Default|GetHealthComponent)) 0.0)
        (Variables|Default|SetIsDead true)
        (Default|CallOnDeath)
        (return true)
        (elif (or (Variables|Default|GetIsInterruptuble) _shouldforceinterrupt)
          (Default|CallOnDamageResponse _damageresponse DamageCauser)
          (return true))))
    (:NoDamage
      (return false))))

(fn ReserveAttackToken
  (params (Amount :type Integer))
  (if (> (Variables|Default|GetTokenCount) 0)
    (Variables|Default|SetTokenCount (- (Variables|Default|GetTokenCount) Amount))
    (return true)
    (else
      (return false))))

(fn ReturnAttackToken
  (params (Amount :type Integer))
  (bind _output_get (Variables|Default|SetTokenCount (+ (Variables|Default|GetTokenCount) Amount)))
  (Development|PrintString (Utilities|String|Append "Token Returned, actual tokens:" (Utilities|String|ToString(Integer) _output_get))))