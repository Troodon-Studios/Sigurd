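; Projectile actor that delivers damage on capsule overlap and destroys itself after a short lifetime.
; It ignores its owner and same-side actors, telling sides apart by whether owner and target each cast to BaseEnemy.
; Targets with the checked component receive DamageInfo through a damageable message, and accepted damage destroys the projectile.
; Rejected damage or other non-Weapon hits spawn sparkles and a crack decal before destroying it.
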(event OnComponentBeginOverlap(Capsule)
  (params (OverlappedComponent :type Primitive%20Component%20Object%20Reference) (OtherActor :type Actor%20Object%20Reference) (OtherComp :type Primitive%20Component%20Object%20Reference) (OtherBodyIndex :type Integer) (bFromSweep :type Boolean) (SweepResult :type Hit%20Result%20Structure%20%28by%20ref%29))
  (bind _returnvalue (Components|GetOwner))
  (if (and (!= OtherActor _returnvalue) (!= (.bSuccess (Utilities|Casting|CastToBaseEnemy _returnvalue)) (.bSuccess (Utilities|Casting|CastToBaseEnemy OtherActor))))
    (Utilities|IsValid (Actor|GetComponentbyClass OtherActor 0)
      (:Is%20Valid
        (bind _wasdamaged (Class|BPIDamageable|TakeDamageDamageable(Message) OtherActor (Variables|Default|GetDamage%20Info) _returnvalue))
        (if _wasdamaged
          (Actor|DestroyActor)
          (else
            (Niagara|SpawnSystematLocation "/Game/VFX/NS_Sparkles.NS_Sparkles" (Transformation|GetActorLocation) :!label _label)
            (bind (_impactpoint _normalrot) (CallFunction|GetDecalLocation self))
            (CallFunction|SpawnDecal "/Game/yTemp/VFX/Decals/DDT_Cracks.DDT_Cracks" _impactpoint _normalrot)
            (Actor|DestroyActor))))
      (:Is%20Not%20Valid
        ;[1 1 1] TODO Debug eliminar esto
        (Utilities|Casting|CastToWeapon OtherActor
          (:CastFailed
            (goto _label)))))))

(event EventBeginPlay
  (Variables|Default|SetTimeAlive 0.0))

(event EventTick
  (params (DeltaSeconds :type Float%20%28single-precision%29))
  (bind _output_get (Variables|Default|SetTimeAlive (+ DeltaSeconds (Variables|Default|GetTimeAlive))))
  (if (>= _output_get 2.0)
    (Actor|DestroyActor)))

(fn ConstructionScript)